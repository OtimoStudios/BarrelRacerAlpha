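; Finish line actor for a race that assigns finishing places from first to fourth as the player and opponents overlap it.
; A shared Place counter is written to the arriving PlayerCharacterBP or OpponentBP, then increments until it reaches fourth.
; The player is also flagged to slow down on crossing.
; Each class branch has a single DoOnce with no reset, so only the first player and first opponent to cross receive a place.
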(event `self.ReceiveActorBeginOverlap`
  (params (OtherActor :type "Actor Object Reference"))
  (`|ExecutionSequence`
    (:`then_0`
      (bind _asplayer_character_bp (cast `/Game/PlayerCharacter/PlayerCharacterBP` OtherActor))
      (`/Engine/EditorBlueprintResources/StandardMacros.DoOnce` false
        (:`Completed`
          (set `/Game/PlayerCharacter/PlayerCharacterBP.SlowDown` true _asplayer_character_bp)
          (switch `int` (`self.Place`)
            (:`1`
              (set `/Game/PlayerCharacter/PlayerCharacterBP.PlaceFinished` 1 _asplayer_character_bp)
              (set `self.Place` (+ (`self.Place`) 1) :!label _label))
            (:`2`
              (set `/Game/PlayerCharacter/PlayerCharacterBP.PlaceFinished` 2 _asplayer_character_bp)
              (goto _label))
            (:`3`
              (set `/Game/PlayerCharacter/PlayerCharacterBP.PlaceFinished` 3 _asplayer_character_bp)
              (goto _label))
            (:`4`
              (set `/Game/PlayerCharacter/PlayerCharacterBP.PlaceFinished` 4 _asplayer_character_bp))))))
    (:`then_1`
      (bind _asopponent_bp (cast `/Game/Opponent/OpponentBP` OtherActor))
      (`/Engine/EditorBlueprintResources/StandardMacros.DoOnce` false
        (:`Completed`
          (switch `int` (`self.Place`)
            (:`1`
              (set `/Game/Opponent/OpponentBP.OpponentFinishedPlace` 1 _asopponent_bp)
              (goto _label))
            (:`2`
              (set `/Game/Opponent/OpponentBP.OpponentFinishedPlace` 2 _asopponent_bp)
              (goto _label))
            (:`3`
              (set `/Game/Opponent/OpponentBP.OpponentFinishedPlace` 3 _asopponent_bp)
              (goto _label))
            (:`4`
              (set `/Game/Opponent/OpponentBP.OpponentFinishedPlace` 4 _asopponent_bp))))))))

(fn `UserConstructionScript`)