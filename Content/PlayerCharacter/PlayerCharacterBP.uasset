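; Player character that parachutes down, then rolls forward automatically over sloped ground, with timed parachute cutting and manual braking.
; Tick drives falling, countdown and rolling; landing switches to Walking after an AirTime check.
; Slope pitch from successive positions feeds curves that set interpolated speed and capsule rotation, with separate flat-ground adjustments.
; Obstacle overlaps reduce health, with knockback from blocks and a camera-fade respawn at zero health.
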(event `InputAction|ParachuteCut`
  (params (Key :type "Key Structure"))
  ;[1 0.4148 0] Activating Parachute
  (:`Pressed`
    (`/Engine/EditorBlueprintResources/StandardMacros.DoOnce` false
      (:`Completed`
        (if (<= (`self.Countdown`) 0.4)
          (set `self.ParachuteRemoved` true)
          (else
            (`KismetSystemLibrary.PrintString` "NOOOOOOOOOO" true true (struct :`R` 1.0 :`A` 1.0))))))))

(event `self.OnLanded`
  (params (Hit :type "HitResult Structure (by ref)"))
  (bind _charactermovement (`self.CharacterMovement`))
  ;[0.01481 1 0.06989] If Landed it Enables Movement
  (set `self.Landed` true)
  (if (>= (`self.AirTime`) 175.0)
    (`KismetSystemLibrary.PrintString` "Killed")
    (elif (and (<= (`self.AirTime`) 174.0) (>= (`self.AirTime`) 150.0))
      (`KismetSystemLibrary.PrintString` "Damage")
      (`CharacterMovementComponent.SetMovementMode` (`self.CharacterMovement`) "MOVE_Walking" 0 :!label _label)
      (set `self.PreviousLocation` (`self.K2_GetActorLocation`))
      (set `CharacterMovementComponent.BrakingDecelerationFalling` 0.0 (`self.CharacterMovement`))
      (set `self.ParachuteRemoved` true)
      (set `CharacterMovementComponent.BrakingDecelerationWalking` 200.0 _charactermovement)
      (set `CharacterMovementComponent.MaxWalkSpeed` 100.0 _charactermovement)
      (set `self.Move` true)
      (elif (<= (`self.AirTime`) 149.0)
        (`KismetSystemLibrary.PrintString` "Good Landing")
        (goto _label)))))

(event `InputAction|Breaking`
  (params (Key :type "Key Structure"))
  ;[1 0 0.1682] Breaking and Speeding UP
  (:`Pressed`
    (if (`self.Landed`)
      (set `self.Braking` true)
      (set `self.SpeedingUp` false)))
  (:`Released`
    (if (`self.Landed`)
      (set `self.SpeedingUp` true))))

(event `self.ReceiveBeginPlay`
  ;[1 0 0.7849] Start the Game Falling
  (set `self.Landed` false)
  (`CharacterMovementComponent.SetMovementMode` (`self.CharacterMovement`) "MOVE_Falling" 0))

(event `self.ReceiveTick`
  (params (DeltaSeconds :type "Float (single-precision)"))
  (bind _countdown (`self.Countdown`))
  (bind _charactermovement (`self.CharacterMovement`))
  (bind _charactermovement_2 (`self.CharacterMovement`))
  (bind _charactermovement_3 (`self.CharacterMovement`))
  (bind _pitch (.pitch (`KismetMathLibrary.FindLookAtRotation` (`self.PreviousLocation`) (`self.K2_GetActorLocation`))))
  (set `self.DeltaTime` DeltaSeconds)
  (`|ExecutionSequence`
    (:`then_0`
      (if (`self.Move`)
        (if (`self.ToBeKnockedBack`)
          (`SceneComponent.K2_SetWorldRotation` (`self.CapsuleComponent`) (`self.PreviousRotation`) false false)
          (`self.AddMovementInput` (`KismetMathLibrary.Conv_RotatorToVector` (`SceneComponent.K2_GetComponentRotation` (`self.CapsuleComponent`))) -1.0)
          (set `CharacterMovementComponent.MaxWalkSpeed` 0.0 _charactermovement_2)
          (`CharacterMovementComponent.SetMovementMode` _charactermovement_2 "MOVE_Walking" 0)
          (`self.AddMovementInput` (`KismetMathLibrary.Conv_RotatorToVector` (`SceneComponent.K2_GetComponentRotation` (`self.CapsuleComponent`))) -100.0 true)
          (set `CharacterMovementComponent.MaxWalkSpeed` 500.0 _charactermovement_2)
          (`KismetSystemLibrary.Delay` 1.5)
          (set `self.ToBeKnockedBack` false)
          (else
            (`self.AddMovementInput` (`KismetMathLibrary.Conv_RotatorToVector` (`self.PreviousRotation`)))
            (if (`self.SlowDown`)
              (`KismetSystemLibrary.PrintString` "Active" false false)
              (`self.SlowDownChar`)
              (`self.UpdateCharRotation`)
              (`KismetSystemLibrary.PrintString` "Hello")
              (elif (`self.Braking`)
                (if (`self.SpeedingUp`)
                  (`|ExecutionSequence`
                    (:`then_0`
                      (`KismetSystemLibrary.Delay` 0.2)
                      (`self.SpeedUp`))
                    (:`then_1`
                      (`self.UpdateCharRotation`))
                    (:`then_2`
                      (if (<= (`CharacterMovementComponent.BrakingDecelerationWalking` (`self.CharacterMovement`)) 10.0)
                        (set `self.SpeedingUp` false)
                        (set `self.Braking` false))))
                  (else
                    (`|ExecutionSequence`
                      (:`then_0`
                        (`self.UpdateCharRotation`))
                      (:`then_1`
                        (`KismetSystemLibrary.Delay` 0.2)
                        (`self.BreakSpeed`)))))
                (elif (and (== _pitch 0.0) (> (`CharacterMovementComponent.MaxWalkSpeed` _charactermovement_3) 400.0))
                  (set `self.PreviousLocation` (`self.K2_GetActorLocation`))
                  (`self.UpdateCharRotation`)
                  (`/Engine/EditorBlueprintResources/StandardMacros.DoOnce` false :!label _label_2
                    (:`Completed`
                      (bind _output_get (set `CharacterMovementComponent.MaxWalkSpeed` (- (`CharacterMovementComponent.MaxWalkSpeed` (`self.CharacterMovement`)) 15.0) _charactermovement_3))
                      (`KismetSystemLibrary.PrintString` (`KismetStringLibrary.Conv_DoubleToString` _output_get) false false)
                      (`KismetSystemLibrary.Delay` 0.5)
                      (goto _label_2 :!via `Reset`)))
                  (elif (and (== _pitch 0.0) (< (`CharacterMovementComponent.MaxWalkSpeed` (`self.CharacterMovement`)) 300.0))
                    (set `self.PreviousLocation` (`self.K2_GetActorLocation`))
                    (`/Engine/EditorBlueprintResources/StandardMacros.DoOnce` false :!label _label_3
                      (:`Completed`
                        (bind _output_get_2 (set `CharacterMovementComponent.MaxWalkSpeed` (+ (`CharacterMovementComponent.MaxWalkSpeed` _charactermovement) 10.0) _charactermovement))
                        (`KismetSystemLibrary.PrintString` (`KismetStringLibrary.Conv_DoubleToString` _output_get_2) false false)
                        (`KismetSystemLibrary.Delay` 0.5)
                        (goto _label_3 :!via `Reset`)))
                    (else
                      (`KismetSystemLibrary.PrintString` (`KismetStringLibrary.Conv_DoubleToString` _pitch) false false)
                      (set `CharacterMovementComponent.BrakingDecelerationWalking` 10.0 (`self.CharacterMovement`))
                      (`self.UpdateCharSpeed`)
                      (`self.UpdateCharRotation`))))))))))
    (:`then_1`
      (if (`NavMovementComponent.IsFalling` (`self.CharacterMovement`))
        (if (`self.ParachuteRemoved`)
          (`KismetSystemLibrary.Delay` 0.2)
          (bind _output_get_3 (set `MovementComponent.Velocity` (- (`self.GetVelocity`) (0.0 0.0 100.0)) (`self.CharacterMovement`)))
          (`KismetSystemLibrary.PrintString` (`KismetStringLibrary.Conv_VectorToString` _output_get_3) false false (struct :`R` 1.0 :`G` 0.038562 :`A` 1.0))
          (else
            (set `CharacterMovementComponent.GravityScale` 0.0 (`self.CharacterMovement`))
            (bind _output_get_4 (set `MovementComponent.Velocity` (0.0 0.0 -300.0) (`self.CharacterMovement`)))
            (`KismetSystemLibrary.PrintString` (`KismetStringLibrary.Conv_VectorToString` _output_get_4) false false (struct :`R` 1.0 :`G` 0.038562 :`A` 1.0))))))
    (:`then_2`
      (if (<= (`self.Countdown`) 0.0)
        (bind _output_get_5 (set `self.Countdown` 0.0))
        (`KismetSystemLibrary.PrintString` (`KismetStringLibrary.Conv_DoubleToString` _output_get_5) false false (struct :`R` 0.033502 :`G` 1.0 :`A` 1.0))
        (else
          (`KismetSystemLibrary.Delay` 0.1)
          (bind _output_get_6 (set `self.Countdown` (`KismetStringLibrary.Conv_StringToDouble` (`KismetTextLibrary.Conv_TextToString` (`KismetTextLibrary.Conv_DoubleToText` (- _countdown 0.1) "HalfToEven" false 1 324 0 1)))))
          (if (or (== _countdown 3.0) (== _countdown 2.0) (== _countdown 1.0))
            (`KismetSystemLibrary.PrintString` (`KismetStringLibrary.Conv_DoubleToString` _output_get_6) false false (struct :`R` 0.033502 :`G` 1.0 :`A` 1.0))))))
    (:`then_3`
      (`KismetSystemLibrary.PrintString` (`KismetStringLibrary.Conv_IntToString` (`self.PlaceFinished`))))))

(event `InputAxis|RollAcelleraction`
  (params (AxisValue :type "Float (single-precision)")))

(event `self.ReceiveActorBeginOverlap`
  (params (OtherActor :type "Actor Object Reference"))
  (`|ExecutionSequence`
    (:`then_0`
      (cast `/Game/Obstacles/BlockObstacle` OtherActor)
      (if (not (`self.ToBeKnockedBack`))
        (`/Engine/EditorBlueprintResources/StandardMacros.DoOnce` false :!label _label_4
          (:`Completed`
            (set `self.ToBeKnockedBack` true)
            (`KismetSystemLibrary.PrintString` "Hit")
            (bind _output_get (set `self.CurrentHealth` (- (`self.CurrentHealth`) 0.05)))
            (`/Engine/EditorBlueprintResources/StandardMacros.CompareFloat` _output_get
              (:`==`
                _)
              (:`<`
                _))
            (`/Engine/EditorBlueprintResources/StandardMacros.DoOnce` false :!label _label_5
              (:`Completed`
                (`self.AddMovementInput` (`KismetMathLibrary.Conv_RotatorToVector` (`SceneComponent.K2_GetComponentRotation` (`self.CapsuleComponent`))) 0.0)
                (`PlayerCameraManager.StartCameraFade` :`self` (`GameplayStatics.GetPlayerCameraManager` 0) :`ToAlpha` 5.0 :`Duration` 3.0)
                (`KismetSystemLibrary.Delay` 3.0)
                (`self.K2_DestroyActor`)
                (`self.RespawnPlayer` (`self.SpawnTransform`))
                (`PlayerCameraManager.StartCameraFade` :`self` (`GameplayStatics.GetPlayerCameraManager` 0) :`FromAlpha` 5.0 :`Duration` 3.0)
                (`KismetSystemLibrary.Delay` 3.0)
                (`self.AddMovementInput` (`KismetMathLibrary.Conv_RotatorToVector` (`SceneComponent.K2_GetComponentRotation` (`self.CapsuleComponent`))))
                (goto _label_5 :!via `Reset`)))))))
    (:`then_1`
      (cast `/Game/Obstacles/DamagingObstacle` OtherActor)
      (bind _output_get_2 (set `self.CurrentHealth` (- (`self.CurrentHealth`) 0.05)))
      (`/Engine/EditorBlueprintResources/StandardMacros.CompareFloat` _output_get_2
        (:`==`
          (goto _label_5))
        (:`<`
          (goto _label_5))))
    (:`then_2`
      (bind _asbreakable_object_bp (cast `/Game/Obstacles/BreakableObjectBP` OtherActor))
      (`GameplayStatics.ApplyDamage` _asbreakable_object_bp 1.0)
      (bind _output_get_3 (set `self.CurrentHealth` (- (`self.CurrentHealth`) 0.3)))
      (`/Engine/EditorBlueprintResources/StandardMacros.CompareFloat` _output_get_3
        (:`==`
          (goto _label_5))
        (:`<`
          (goto _label_5))))
    (:`then_3`
      (bind _aschance_cube_bp (cast `/Game/PickUpSystem/chanceCubeBP` OtherActor))
      (`self.K2_DestroyActor` _aschance_cube_bp))))

(event `InputAxis|Turn`
  (params (AxisValue :type "Float (single-precision)")))

(event `self.ReceiveActorEndOverlap`
  (params (OtherActor :type "Actor Object Reference"))
  (`|ExecutionSequence`
    (:`then_0`
      (cast `/Game/Obstacles/BlockObstacle` OtherActor)
      (goto _label_4 :!via `Reset`))))

(fn `BreakSpeed`
  (bind _charactermovement (`self.CharacterMovement`))
  (bind _brakingdecelerationwalking (`CharacterMovementComponent.BrakingDecelerationWalking` _charactermovement))
  (bind _maxwalkspeed (`CharacterMovementComponent.MaxWalkSpeed` _charactermovement))
  (if (`self.Braking`)
    (`|ExecutionSequence`
      (:`then_0`
        (if (not (>= _brakingdecelerationwalking 300.0))
          (`/Engine/EditorBlueprintResources/StandardMacros.DoOnce` false :!label _label
            (:`Completed`
              (bind _output_get (set `CharacterMovementComponent.BrakingDecelerationWalking` (+ _brakingdecelerationwalking 10.0) _charactermovement))
              (`KismetSystemLibrary.PrintString` (`KismetStringLibrary.Conv_DoubleToString` _output_get) false false (struct :`R` 1.0 :`G` 0.063568 :`A` 1.0))
              (goto _label :!via `Reset`)))))
      (:`then_1`
        (if (>= _maxwalkspeed 200.0)
          (`/Engine/EditorBlueprintResources/StandardMacros.DoOnce` false :!label _label_2
            (:`Completed`
              (bind _output_get_2 (set `CharacterMovementComponent.MaxWalkSpeed` (- _maxwalkspeed 10.0) _charactermovement))
              (`KismetSystemLibrary.PrintString` (`KismetStringLibrary.Conv_DoubleToString` _output_get_2) false false (struct :`G` 0.001571 :`B` 1.0 :`A` 1.0))
              (goto _label_2 :!via `Reset`))))))))

(fn `GetSpeedAngle`
  (returns (DesiredSpeed :type "Float (double-precision)") (NewParam :type "Rotator Structure"))
  (locals (Speed :type "Float (double-precision)" :default 0.0))
  (bind _pitch (.pitch (`KismetMathLibrary.FindLookAtRotation` (`self.PreviousLocation`) (`self.K2_GetActorLocation`))))
  ;[1 1 1] Get Angel Speed - Get Floor angel- Get value from curve
  (set `self.Rotation` (`KismetMathLibrary.MakeRotator` 0.0 (`CurveFloat.GetFloatValue` (`self.SlopeRotation`) _pitch)))
  (set `local.Speed` (`CurveFloat.GetFloatValue` (`self.SpeedCurve`) _pitch))
  (set `self.PreviousLocation` (`self.K2_GetActorLocation`))
  (return (`local.Speed`) (`self.Rotation`)))

(fn `RespawnPlayer`
  (params (Transform :type "Transform Structure"))
  (bind _returnvalue (`|SpawnActorFromClass` "PlayerCharacterBP_C" Transform "Undefined" "OverrideRootScale" null null))
  (`Controller.Possess` (`GameplayStatics.GetPlayerController` 0) _returnvalue))

(fn `RotateCharacter`
  (bind _returnvalue (`KismetMathLibrary.MakeRotator` 0.0 (* (.pitch (`self.Rotation`)) -1.0) (+ (.yaw (`self.PreviousRotation`)) (`self.GetInputAxisValue`))))
  (bind _returnvalue_2 (`KismetMathLibrary.RInterpTo` _returnvalue (`SceneComponent.K2_GetComponentRotation` (`self.CapsuleComponent`)) (`self.DeltaTime`) 5.0))
  (`KismetSystemLibrary.PrintString` (`KismetStringLibrary.Conv_RotatorToString` _returnvalue_2) false false)
  (set `self.PreviousRotation` _returnvalue)
  (`SceneComponent.K2_SetWorldRotation` (`self.CapsuleComponent`) _returnvalue_2 false false))

(fn `ShouldUpdateRotation`
  (returns (CanTurn :type Boolean))
  (bind _charactermovement (`self.CharacterMovement`))
  (bind _returnvalue (and (not (`NavMovementComponent.IsFalling` _charactermovement)) (> (`KismetMathLibrary.VSizeSquared` (`MovementComponent.Velocity` _charactermovement)) 0.0) (<= (`CharacterMovementComponent.BrakingDecelerationWalking` _charactermovement) 300.0)))
  (`KismetSystemLibrary.PrintString` (`KismetStringLibrary.Conv_BoolToString` _returnvalue) false false)
  (return _returnvalue))

(fn `ShouldUpdateSpeed`
  (returns (ShouldUpdate :type Boolean))
  (bind _charactermovement (`self.CharacterMovement`))
  (bind _returnvalue (and (not (`NavMovementComponent.IsFalling` _charactermovement)) (> (`KismetMathLibrary.VSizeSquared` (`MovementComponent.Velocity` _charactermovement)) 0.0)))
  ;[1 1 1] Should Update - On the ground - Have Velocity
  (`KismetSystemLibrary.PrintString` (`KismetStringLibrary.Conv_BoolToString` _returnvalue) false false)
  (return _returnvalue))

(fn `SlowDownChar`
  (bind _charactermovement (`self.CharacterMovement`))
  (bind _maxwalkspeed (`CharacterMovementComponent.MaxWalkSpeed` _charactermovement))
  (bind _brakingdecelerationwalking (`CharacterMovementComponent.BrakingDecelerationWalking` _charactermovement))
  (bind _returnvalue (`KismetMathLibrary.RInterpTo` (`SceneComponent.K2_GetComponentRotation` (`self.CapsuleComponent`)) (`self.Rotation`) 0.0 (`KismetMathLibrary.MapRangeClamped` (.pitch (`self.Rotation`)) 0.0 90.0 1.0 3.0)))
  (`|ExecutionSequence`
    (:`then_0`
      (if (<= _maxwalkspeed 0.0)
        (set `CharacterMovementComponent.MaxWalkSpeed` 0.0 _charactermovement)
        (else
          (`/Engine/EditorBlueprintResources/StandardMacros.DoOnce` false :!label _label
            (:`Completed`
              (set `CharacterMovementComponent.MaxWalkSpeed` (- _maxwalkspeed 10.0) _charactermovement)
              (`KismetSystemLibrary.PrintString` (`KismetStringLibrary.Conv_DoubleToString` _maxwalkspeed) false false)
              (goto _label :!via `Reset`))))))
    (:`then_1`
      (if (== _brakingdecelerationwalking 2840.0)
        (set `CharacterMovementComponent.BrakingDecelerationWalking` 2840.0 _charactermovement)
        (else
          (`/Engine/EditorBlueprintResources/StandardMacros.DoOnce` false :!label _label_2
            (:`Completed`
              (set `CharacterMovementComponent.BrakingDecelerationWalking` (+ _brakingdecelerationwalking 2.0) _charactermovement)
              (`KismetSystemLibrary.PrintString` (`KismetStringLibrary.Conv_DoubleToString` _brakingdecelerationwalking) false false)
              (goto _label_2 :!via `Reset`))))))
    (:`then_2`
      (set `self.Rotation` (`KismetMathLibrary.MakeRotator` 0.0 (`CurveFloat.GetFloatValue` (`self.SlopeRotation`) (.pitch (`KismetMathLibrary.FindLookAtRotation` (`self.PreviousLocation`) (`self.K2_GetActorLocation`))))))
      (set `self.PreviousLocation` (`self.K2_GetActorLocation`))
      (`SceneComponent.K2_SetWorldRotation` (`self.CapsuleComponent`) _returnvalue false false)
      (`KismetSystemLibrary.PrintString` (`KismetStringLibrary.Conv_RotatorToString` _returnvalue) false false))))

(fn `SpeedUp`
  (bind _charactermovement (`self.CharacterMovement`))
  (bind _brakingdecelerationwalking (`CharacterMovementComponent.BrakingDecelerationWalking` _charactermovement))
  (bind _maxwalkspeed (`CharacterMovementComponent.MaxWalkSpeed` _charactermovement))
  (`|ExecutionSequence`
    (:`then_0`
      (if (not (<= _brakingdecelerationwalking 10.0))
        (`/Engine/EditorBlueprintResources/StandardMacros.DoOnce` false :!label _label
          (:`Completed`
            (bind _output_get (set `CharacterMovementComponent.BrakingDecelerationWalking` (- _brakingdecelerationwalking 10.0) _charactermovement))
            (`KismetSystemLibrary.PrintString` (`KismetStringLibrary.Conv_DoubleToString` _output_get) false false (struct :`R` 0.012519 :`G` 1.0 :`A` 1.0))
            (goto _label :!via `Reset`)))))
    (:`then_1`
      (if (>= _maxwalkspeed 150.0)
        (`/Engine/EditorBlueprintResources/StandardMacros.DoOnce` false :!label _label_2
          (:`Completed`
            (bind _output_get_2 (set `CharacterMovementComponent.MaxWalkSpeed` (+ _maxwalkspeed 10.0) _charactermovement))
            (`KismetSystemLibrary.PrintString` (`KismetStringLibrary.Conv_DoubleToString` _output_get_2) false false (struct :`G` 0.001571 :`B` 1.0 :`A` 1.0))
            (goto _label_2 :!via `Reset`)))))))

(fn `UpdateCharRotation`
  (bind _canturn (`self.ShouldUpdateRotation`))
  (if _canturn
    (`self.RotateCharacter`)
    (else
      (`SceneComponent.K2_SetWorldRotation` (`self.CapsuleComponent`) (`self.PreviousRotation`) false false))))

(fn `UpdateCharSpeed`
  ;[1 1 1] Update Character Speed- Should Update- Get Speed Angle - Update Movement Speed
  (`KismetSystemLibrary.PrintString` (`KismetStringLibrary.Conv_DoubleToString` (`CharacterMovementComponent.MaxWalkSpeed` (`self.CharacterMovement`))) false false)
  (bind _shouldupdate (`self.ShouldUpdateSpeed`))
  (if _shouldupdate
    (bind (_desiredspeed _newparam) (`self.GetSpeedAngle`))
    (`self.UpdateMovementSpeed` _desiredspeed _newparam)
    (else
      ;;[0.004949 1 0.01923] Testing
      (`CharacterMovementComponent.SetMovementMode` (`self.CharacterMovement`) "MOVE_Falling" 0))))

(fn `UpdateMovementSpeed`
  (params (DesiredSpeed :type "Float (double-precision)") (DesiredRotation :type "Rotator Structure"))
  (bind _deltatime (`self.DeltaTime`))
  ;[1 1 1] Interp to desired speed
  (bind _output_get (set `CharacterMovementComponent.MaxWalkSpeed` (`KismetMathLibrary.FInterpTo` (`CharacterMovementComponent.MaxWalkSpeed` (`self.CharacterMovement`)) DesiredSpeed _deltatime (`KismetMathLibrary.MapRangeClamped` DesiredSpeed 100.0 900.0 1.0 6.0)) (`self.CharacterMovement`)))
  (`SceneComponent.K2_SetWorldRotation` (`self.CapsuleComponent`) (`KismetMathLibrary.RInterpTo` (`SceneComponent.K2_GetComponentRotation` (`self.CapsuleComponent`)) DesiredRotation _deltatime (`KismetMathLibrary.MapRangeClamped` (.pitch DesiredRotation) 0.0 90.0 5.0 5.0)) false false)
  (`KismetSystemLibrary.PrintString` (`KismetStringLibrary.Conv_DoubleToString` _output_get) false false (struct :`R` 0.078006 :`G` 1.0 :`A` 1.0)))

(fn `UserConstructionScript`)